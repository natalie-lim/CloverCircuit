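; BP_FarmerNPC is a farmer NPC that opens a dialogue when the first-person player enters its dialogue collision box.
; Each player overlap creates and stores a farmer dialogue widget, adds it to the viewport, and switches to Game and UI input with a visible cursor.
; An AlreadyInteracted flag limits disabling player input to the first encounter; this Blueprint does not re-enable input or remove the widget.
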(event `self.Box_DialogueCollision.OnComponentBeginOverlap`
  (params (OverlappedComponent :type "PrimitiveComponent Object Reference") (OtherActor :type "Actor Object Reference") (OtherComp :type "PrimitiveComponent Object Reference") (OtherBodyIndex :type Integer) (bFromSweep :type Boolean) (SweepResult :type "HitResult Structure (by ref)"))
  (bind _asbp_first_person_character (cast `/Game/FirstPerson/Blueprints/BP_FirstPersonCharacter` OtherActor))
  (bind _returnvalue (`|CreateWidget` "/Game/UI/WBP_FarmerDialogue.WBP_FarmerDialogue_C"))
  (set `self.DialogueWidgetRef` _returnvalue)
  (`UserWidget.AddToViewport` _returnvalue 0)
  (bind _returnvalue_2 (`PlayerState.GetPlayerController` (`Pawn.PlayerState` _asbp_first_person_character)))
  (`WidgetBlueprintLibrary.SetInputMode_GameAndUIEx` _returnvalue_2 null "DoNotLock" false)
  (set `PlayerController.bShowMouseCursor` true _returnvalue_2)
  (if (not (`self.bAlreadyInteracted`))
    (`self.DisableInput` _asbp_first_person_character _returnvalue_2)
    (set `self.bAlreadyInteracted` true)))

(fn `UserConstructionScript`)