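; An inventory component that stores items and quantities as an array of inventory slots.
; AddItem matches items by ItemID, increases the matching slot's quantity, and prints the new amount.
; The AlrThere flag is set false on a match, so the following check can still append a new slot.
; RemoveItem is an empty stub, and BeginPlay and Tick are unused.
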(fn `AddItem`
  (params (Item :type "/Game/Inventory/BP_InventoryItemAsset Object Reference") (Amount :type Integer))
  (returns (Inventory :type "Array of /Game/Inventory/InventorySlot Structure"))
  (bind (_itemdata_displayname _itemdata_icon _itemdata_itemid) (break `/Game/Inventory/InventoryItemData` (`/Game/Inventory/BP_InventoryItemAsset.ItemData` Item)))
  (bind _inventory (`self.Inventory`))
  (for (_array_element _array_index) _inventory
    (bind (_item _quantity) (break `/Game/Inventory/InventorySlot` _array_element))
    (bind (_itemdata_displayname_2 _itemdata_icon_2 _itemdata_itemid_2) (break `/Game/Inventory/InventoryItemData` (`/Game/Inventory/BP_InventoryItemAsset.ItemData` _item)))
    (if (== _itemdata_itemid_2 _itemdata_itemid)
      (set `self.bAlrThere` false)
      (bind _returnvalue (+ Amount _quantity))
      (`KismetArrayLibrary.Array_Set` (`self.Inventory`) _array_index (make `/Game/Inventory/InventorySlot` Item _returnvalue))
      (`KismetSystemLibrary.PrintString` "new amount: ")
      (`KismetSystemLibrary.PrintString` (`KismetStringLibrary.Conv_IntToString` _returnvalue))))
  (if (not (`self.bAlrThere`))
    (`KismetArrayLibrary.Array_Add` _inventory (make `/Game/Inventory/InventorySlot` Item Amount)))
  (return (`self.Inventory`)))

(fn `RemoveItem`)